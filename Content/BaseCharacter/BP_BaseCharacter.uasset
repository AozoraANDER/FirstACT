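; Player base character that handles Enhanced Input movement, camera, sprint and samurai melee actions.
; A timeline ramps walk speed for running, defense cancels the run, and Tick toggles orient-to-movement by velocity.
; A one-time equip montage unlocks directional dodges, backward by default, and a five-step attack combo.
; State flags gate these montages; dodge clears after a delay, while attack relies on separate reset and combo-end events.
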(event `self.ReceiveBeginPlay`
  ;[1 1 1] Load Import Mapping
  (bind _asplayer_controller (cast `PlayerController` (`self.GetController`)))
  (bind _returnvalue (pcsubsystem `EnhancedInputLocalPlayerSubsystem` _asplayer_controller))
  (`/Engine/EditorBlueprintResources/StandardMacros.IsValid` _returnvalue
    (:`Is Valid`
      (`EnhancedInputSubsystemInterface.AddMappingContext` _returnvalue "/Game/Input/IMC_BaseInputMapping.IMC_BaseInputMapping" 0 (struct)))))

(event `EnhancedInput|/Game/Input/IA_Equip`
  (params (ActionValue :type Boolean) (ElapsedSeconds :type "Float (double-precision)") (TriggeredSeconds :type "Float (double-precision)") (InputAction :type "InputAction Object Reference" :default "/Game/Input/IA_Equip.IA_Equip"))
  ;[1 1 1] Equip
  (:`Started`
    (`/Engine/EditorBlueprintResources/StandardMacros.DoOnce` false
      (:`Completed`
        (`AnimInstance.Montage_Play` (`SkeletalMeshComponent.GetAnimInstance` (`self.Mesh`)) (select `int` (`KismetMathLibrary.RandomIntegerInRange` 0 1) :`0` "/Game/Pawn/GhostSamurai_APose_Equip01_Root_Montage.GhostSamurai_APose_Equip01_Root_Montage" :`1` "/Game/Pawn/GhostSamurai_APose_Equip02_Root_Montage.GhostSamurai_APose_Equip02_Root_Montage" :!type "AnimMontage Object Reference") 1.0 "MontageLength" 0.0 true)
        (set `self.Equiped` true)))))

(event `self.ReceiveTick`
  (params (DeltaSeconds :type "Float (single-precision)"))
  (bind _charactermovement (`self.CharacterMovement`))
  ;[1 1 1] Fix the Camera problem
  (if (> (`KismetMathLibrary.VSize` (`self.GetVelocity`)) 0.0)
    (set `CharacterMovementComponent.bOrientRotationToMovement` false _charactermovement)
    (else
      (set `CharacterMovementComponent.bOrientRotationToMovement` true _charactermovement))))

(event `EnhancedInput|/Game/Input/IA_Look`
  (params (ActionValue :type "Vector2D Structure") (ElapsedSeconds :type "Float (double-precision)") (TriggeredSeconds :type "Float (double-precision)") (InputAction :type "InputAction Object Reference" :default "/Game/Input/IA_Look.IA_Look"))
  (bind (_x _y) (`KismetMathLibrary.BreakVector2D` ActionValue))
  ;[1 1 1] Camera Moving
  (:`Triggered`
    (`self.AddControllerYawInput` _x)
    (`self.AddControllerPitchInput` _y)))

(event `EnhancedInput|/Game/Input/IA_Move`
  (params (ActionValue :type "Vector2D Structure") (ElapsedSeconds :type "Float (double-precision)") (TriggeredSeconds :type "Float (double-precision)") (InputAction :type "InputAction Object Reference" :default "/Game/Input/IA_Move.IA_Move"))
  (bind (_x _y) (`KismetMathLibrary.BreakVector2D` ActionValue))
  (bind (_returnvalue_roll _returnvalue_pitch _returnvalue_yaw) (`KismetMathLibrary.BreakRotator` (`self.GetControlRotation`)))
  ;[1 1 1] Movement
  (:`Triggered`
    (`self.AddMovementInput` (`KismetMathLibrary.GetRightVector` (`KismetMathLibrary.MakeRotator` _returnvalue_roll 0.0 _returnvalue_yaw)) _x)
    (`self.AddMovementInput` (`KismetMathLibrary.GetForwardVector` (`KismetMathLibrary.MakeRotator` 0.0 0.0 _returnvalue_yaw)) _y)))

(event `EnhancedInput|/Game/Input/IA_Run`
  (params (ActionValue :type Boolean) (ElapsedSeconds :type "Float (double-precision)") (TriggeredSeconds :type "Float (double-precision)") (InputAction :type "InputAction Object Reference" :default "/Game/Input/IA_Run.IA_Run"))
  ;[1 1 1] Run
  (:`Started`
    (if (not (`self.Defense`))
      (set `self.Run` true)
      (bind (_direction _speed) (`Timeline|RunSpeed` :!label _label)
        (:`Update`
          (set `CharacterMovementComponent.MaxWalkSpeed` _speed (`self.CharacterMovement`))))))
  (:`Completed`
    (set `self.Run` false :!label _label_2)
    (goto _label :!via `Reverse`)))

(event `EnhancedInput|/Game/Input/IA_Defense`
  (params (ActionValue :type Boolean) (ElapsedSeconds :type "Float (double-precision)") (TriggeredSeconds :type "Float (double-precision)") (InputAction :type "InputAction Object Reference" :default "/Game/Input/IA_Defense.IA_Defense"))
  ;[1 1 1] Defense
  (:`Started`
    (if (`self.Run`)
      (`|ExecutionSequence`
        (:`then_0`
          (goto _label_2))
        (:`then_1`
          _)))
    (set `self.Defense` true))
  (:`Completed`
    (set `self.Defense` false)))

(event `EnhancedInput|/Game/Input/IA_Dodge`
  (params (ActionValue :type Boolean) (ElapsedSeconds :type "Float (double-precision)") (TriggeredSeconds :type "Float (double-precision)") (InputAction :type "InputAction Object Reference" :default "/Game/Input/IA_Dodge.IA_Dodge"))
  (bind (_returnvalue_x _returnvalue_y) (`KismetMathLibrary.BreakVector2D` (`|GetInputActionValue`)))
  (bind _returnvalue (`SkeletalMeshComponent.GetAnimInstance` (`self.Mesh`)))
  ;[1 1 1] Dodge
  (:`Started`
    (if (`self.Equiped`)
      (if (not (`self.DodgeMontagePlay`))
        (set `self.DodgeMontagePlay` true)
        (set `self.bUseControllerRotationYaw` true)
        (if (!= _returnvalue_y 0.0)
          (if (> _returnvalue_y 0.0)
            (`AnimInstance.Montage_Play` _returnvalue "/Game/Pawn/GhostSamurai_APose_Dodge_F_Root_Montage.GhostSamurai_APose_Dodge_F_Root_Montage" 1.2 "MontageLength" 0.0 true)
            (else
              (`AnimInstance.Montage_Play` _returnvalue "/Game/Pawn/GhostSamurai_APose_Dodge_B_Root_Montage.GhostSamurai_APose_Dodge_B_Root_Montage" 1.2 "MontageLength" 0.0 true :!label _label_3)))
          (elif (!= _returnvalue_x 0.0)
            (if (> _returnvalue_x 0.0)
              (`AnimInstance.Montage_Play` _returnvalue "/Game/Pawn/GhostSamurai_APose_Dodge_R_Root_Montage.GhostSamurai_APose_Dodge_R_Root_Montage" 1.2 "MontageLength" 0.0 true)
              (else
                (`AnimInstance.Montage_Play` _returnvalue "/Game/Pawn/GhostSamurai_APose_Dodge_L_Root_Montage.GhostSamurai_APose_Dodge_L_Root_Montage" 1.2 "MontageLength" 0.0 true)))
            (else
              (goto _label_3))))
        (`KismetSystemLibrary.Delay` 0.45)
        (set `self.DodgeMontagePlay` false)
        (set `self.bUseControllerRotationYaw` false)))))

(event `EnhancedInput|/Game/Input/IA_Attack`
  (params (ActionValue :type Boolean) (ElapsedSeconds :type "Float (double-precision)") (TriggeredSeconds :type "Float (double-precision)") (InputAction :type "InputAction Object Reference" :default "/Game/Input/IA_Attack.IA_Attack"))
  (:`Started`
    (if (`self.Equiped`)
      (if (not (or (`self.AttackMontagePlay`) (`self.DodgeMontagePlay`)))
        (set `self.bUseControllerRotationYaw` true)
        (if (== (`self.AttackIndex`) 5)
          (set `self.AttackIndex` 0))
        (set `self.AttackMontagePlay` true)
        (`AnimInstance.Montage_Play` (`SkeletalMeshComponent.GetAnimInstance` (`self.Mesh`)) (`|GetArrayItem` (`self.AttackMontages_0`) (`self.AttackIndex`)) 1.0 "MontageLength" 0.0 true)
        (`/Engine/EditorBlueprintResources/StandardMacros.IncrementInt` (`self.AttackIndex`)
          (:`  `
            (set `self.bUseControllerRotationYaw` false)))))))

(event `ResetAttackMontage`
  (set `self.AttackMontagePlay` false))

(event `EndingCombo`
  (set `self.AttackIndex` 0))

(fn `UserConstructionScript`)